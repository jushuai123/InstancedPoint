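; Point manager actor that spawns a cloud of instanced point meshes and supports mouse picking of individual points.
; On BeginPlay it adds a BPCPoint component with a throttled tick, sets its mesh and bounds, then scatters instances at random directions scaled into a flattened ellipsoid.
; Left click deprojects the cursor into a complex visibility trace and prints the hit item index, or a miss message.
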(event `self.ReceiveBeginPlay`
  (bind _returnvalue (`AddComponent|NODE_AddBPC_Point-0` :`RelativeTransform` (`KismetMathLibrary.MakeTransform` (0.0 0.0 0.0))))
  (`ActorComponent.SetComponentTickInterval` _returnvalue 0.1)
  (`StaticMeshComponent.SetStaticMesh` _returnvalue "/InstancedPoint/SM_PointType.SM_PointType")
  (`InstancedPointComponent.SetBoundsSize` _returnvalue)
  (for _ (range (+ (`self.SpawnLastIndex`) 1))
    (`InstancedStaticMeshComponent.AddInstance` _returnvalue (`KismetMathLibrary.MakeTransform` (* (`KismetMathLibrary.RandomUnitVector`) (500.0 500.0 50.0))))))

(event `Key|LeftMouseButton`
  (params (Key :type "Key Structure"))
  (:`Pressed`
    (bind _returnvalue (`WidgetLayoutLibrary.GetMousePositionOnViewport`))
    (bind (_worldposition _worlddirection _returnvalue_2) (`GameplayStatics.DeprojectScreenToWorld` (`GameplayStatics.GetPlayerController` 0) (* _returnvalue (`WidgetLayoutLibrary.GetViewportScale`))))
    (if _returnvalue_2
      (bind (_outhit _returnvalue_3) (`KismetSystemLibrary.LineTraceSingle` :`Start` _worldposition :`End` (+ _worldposition (* _worlddirection 10000.0)) :`TraceChannel` "TraceTypeQuery1" :`bTraceComplex` true :`bIgnoreSelf` false :`DrawTime` 10.0))
      (if _returnvalue_3
        (`KismetSystemLibrary.PrintString` (`KismetStringLibrary.Conv_IntToString` (`.HitItem` (`GameplayStatics.BreakHitResult` _outhit))))
        (else
          (`KismetSystemLibrary.PrintString` "Not Hit"))))))

(fn `UserConstructionScript`)